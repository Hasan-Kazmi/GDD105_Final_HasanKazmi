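; BP_Door is a door that opens when the player character enters its trigger box and the required number of rune pads are active.
; On each overlap it gathers every BP_RunePad in the level, counts the activated ones and compares the count for exact equality with RequiredRunePads.
; A match plays Door_Timeline, which drives the door's sideways and forward offset and its yaw; no logic closes it.
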(event OnComponentBeginOverlap(BoxCollision)
  (params (OverlappedComponent :type Primitive%20Component%20Object%20Reference) (OtherActor :type Actor%20Object%20Reference) (OtherComp :type Primitive%20Component%20Object%20Reference) (OtherBodyIndex :type Integer) (bFromSweep :type Boolean) (SweepResult :type Hit%20Result%20Structure%20%28by%20ref%29))
  (Utilities|Casting|CastToBP_ThirdPersonCharacter OtherActor)
  (bind _outactors (Actor|GetAllActorsOfClass "/Game/RunePad/BP_RunePad.BP_RunePad_C"))
  (bind _output_get (Variables|Default|SetRunePads _outactors))
  (Variables|Default|SetActivatedRunePads 0)
  (for _array_element _output_get
    (if (Variables|/Game/RunePad/BP_RunePad.BP_RunePad_C|GetIsActivated? _array_element)
      (Math|Integer|IncrementInt (Variables|Default|GetActivatedRunePads))))
  (if (== (Variables|Default|GetRequiredRunePads) (Variables|Default|GetActivatedRunePads))
    (bind (_direction _opening _side_movement _front_movement) (Timeline|Door_Timeline Play)
      (:Update
        (Transformation|SetRelativeLocationAndRotation (Variables|Default|GetDoor) (Math|Vector|MakeVector _side_movement _front_movement 0.0) (Math|Rotator|MakeRotator 0.0 0.0 _opening) false false)))))

(event EventBeginPlay)

(event Collision|EventActorBeginOverlap
  (params (OtherActor :type Actor%20Object%20Reference)))

(event EventTick
  (params (DeltaSeconds :type Float%20%28single-precision%29)))

(fn ConstructionScript)